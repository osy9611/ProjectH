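; BP_Character is a character Blueprint that gives the character dialog and speech bubble access through the UI manager subsystem.
; ShowDialogLine creates WBP_Dialog on the Dialog UI layer and shows a line by table ID, with the character as speaker.
; GetWBPDialog and GetSpeechBubble use the same CreateUI call to return the dialog widget or its WBP_Speech bubble.
; The event graph and construction script are empty, and an unused HUD-based dialog path remains disconnected.
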(fn `GetSpeechBubble`
  (returns (SpeechBubble :type "/Game/Widgets/Dialog/WBP_Speech Object Reference"))
  (bind _returnvalue (`UIManagerSubsystem.CreateUI` (subsystem `UIManagerSubsystem`) (struct :`TagName` "UI.Layer.Dialog") "/Game/Widgets/WBP_Dialog.WBP_Dialog_C"))
  (bind _aswbp_dialog (cast `/Game/Widgets/WBP_Dialog` _returnvalue))
  (bind _aswbp_speech (cast `/Game/Widgets/Dialog/WBP_Speech` (`CommonActivatableWidget_Dialog.SpeechBubbleWidget` _aswbp_dialog)))
  (return _aswbp_speech))

(fn `GetWBPDialog`
  (returns (NewParam :type "/Game/Widgets/WBP_Dialog Object Reference"))
  (bind _returnvalue (`UIManagerSubsystem.CreateUI` (subsystem `UIManagerSubsystem`) (struct :`TagName` "UI.Layer.Dialog") "/Game/Widgets/WBP_Dialog.WBP_Dialog_C"))
  (bind _aswbp_dialog (cast `/Game/Widgets/WBP_Dialog` _returnvalue))
  (return _aswbp_dialog))

(fn `Show Dialog Line`
  (params (DialogID :type Integer))
  (bind _returnvalue (`UIManagerSubsystem.CreateUI` (subsystem `UIManagerSubsystem`) (struct :`TagName` "UI.Layer.Dialog") "/Game/Widgets/WBP_Dialog.WBP_Dialog_C"))
  (bind _aswbp_dialog (cast `/Game/Widgets/WBP_Dialog` _returnvalue))
  (`CommonActivatableWidget_Dialog.ShowDialog` _aswbp_dialog DialogID self)
  (return))

(fn `UserConstructionScript`)