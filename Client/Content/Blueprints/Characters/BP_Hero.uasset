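; Hero character Blueprint that sets up interaction and shares the player's position with materials.
; On BeginPlay it assigns InteractionCheck as the Interaction component's collision, then registers that component through HDHero's RegisterInteractionComponent.
; Every Tick it writes the actor's location to the PlayerPosition parameter of the MPC_Masking Material Parameter Collection, so materials can read it globally.
; The construction script only calls the parent's.
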(event `self.ReceiveBeginPlay`
  (set `InteractionComponent.Collision` (`self.InteractionCheck`) (`self.Interaction`))
  (`HDHeroComponent.RegisterInteractionComponent` (`self.HDHero`) (`self.Interaction`)))

(event `self.ReceiveTick`
  (params (DeltaSeconds :type "Float (single-precision)"))
  (`KismetMaterialLibrary.SetVectorParameterValue` "/Game/Materials/MPC_Masking.MPC_Masking" "PlayerPosition" (`KismetMathLibrary.Conv_VectorToLinearColor` (`self.K2_GetActorLocation`))))

(fn `UserConstructionScript`
  (`parent.UserConstructionScript`))