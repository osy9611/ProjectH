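; NPC character that can roam the navmesh and hold speech-bubble dialogue with an interactor.
; Roaming loops AI moves to random nearby points after random delays, stopping if its interaction lock is set when a delay ends.
; Dialogue events open a line or, while the interactor is locked, finish the text reveal or check for the next line, toggling the indicator.
; SetDir yaws it along the direction from a target to itself.
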(event `self.ReceiveBeginPlay`
  (if (`self.Is Roaming`)
    (bind _randomlocation (`NavigationSystemV1.K2_GetRandomLocationInNavigableRadius` (`self.K2_GetActorLocation`) 1000.0 null null :!label _label))
    (`|AIMoveTo` self _randomlocation null 200.0
      (:`OnSuccess`
        _)
      (:`OnFail`
        _))
    (`self.MoveRandomWithDelay`)))

(event `MoveRandomWithDelay`
  (`KismetSystemLibrary.RetriggerableDelay` (`KismetMathLibrary.RandomFloatInRange` (`self.MinPatrolDelay`) (`self.MaxPatrolDelay`)))
  (bind _returnvalue (`HDPawnExtensionComponent.GetInteractionLock` (`self.PawnExtComponent`)))
  (if (not _returnvalue)
    (goto _label)))

(event `self.HDNPC.OnLoadComplete`
  (params (NPCData :type "NPCData Structure"))
  (if (== NPCData_InteractionValue 0)
    (`SceneComponent.SetVisibility` (`self.DialogueIndicator`) false false)))

(event `self.HDNPC.OnDialog`
  (params (DialogID :type Integer) (Interactor :type "Actor Object Reference"))
  ;[1 1 1] Interaction Dioalog
  (bind _returnvalue (`HDPawnExtensionComponent.GetInteractionLock` (`self.GetComponentByClass` Interactor "/Script/ProjectH.HDPawnExtensionComponent")))
  (if _returnvalue
    (bind _speechbubble (`self.GetSpeechBubble`))
    (bind _returnvalue_2 (`SpeechBubbleWidget.FinishedRevealing` _speechbubble))
    (if _returnvalue_2
      (bind _newparam (`self.GetWBPDialog`))
      (bind _isend (`CommonActivatableWidget_Dialog.CheckNextDialog` _newparam self))
      (if _isend
        (`HDNPCComponent.FinishInteraction` (`self.HDNPC`))
        (`SceneComponent.SetVisibility` (`self.DialogueIndicator`) true false))
      (else
        (`/Game/Widgets/Dialog/WBP_Speech.InstaReveal` _speechbubble)))
    (else
      (`self.Show Dialog Line` DialogID)
      (`SceneComponent.SetVisibility` (`self.DialogueIndicator`) false false))))

(fn `SetDir`
  (params (Target :type "Actor Object Reference"))
  (bind (_returnvalue_roll _returnvalue_pitch) (`KismetMathLibrary.BreakRotator` (`self.K2_GetActorRotation`)))
  (bind (_returnvalue_roll_2 _returnvalue_pitch_2 _returnvalue_yaw) (`KismetMathLibrary.BreakRotator` (`KismetMathLibrary.FindLookAtRotation` (`self.K2_GetActorLocation` Target) (`self.K2_GetActorLocation`))))
  (`self.K2_SetActorRotation` (`KismetMathLibrary.MakeRotator` _returnvalue_roll _returnvalue_pitch _returnvalue_yaw)))

(fn `UserConstructionScript`
  (`parent.UserConstructionScript`))